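; BP_FollowPathCamera is an actor that runs an automated flythrough along a spline, with optional profiling, then quits the game.
; On BeginPlay it finds BP_Spline and BP_LookAtActor, snaps to the spline start and waits briefly.
; A timeline, rate-scaled by TimeToCompleteSec, moves it along the spline's length while keeping it facing the target.
; When Test is set, console commands start profiling before the move and stop it after.
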(event `self.ReceiveBeginPlay`
  (bind _returnvalue (`GameplayStatics.GetActorOfClass` "/Game/Blueprints/BP_Spline.BP_Spline_C"))
  (set `self.spline Ref` _returnvalue)
  (bind _returnvalue_2 (`GameplayStatics.GetActorOfClass` "/Game/Blueprints/BP_LookAtActor.BP_LookAtActor_C"))
  (set `self.LookAtTarget` _returnvalue_2)
  (`self.Move`))

(event `Move`
  (bind _returnvalue (`SplineComponent.GetLocationAtDistanceAlongSpline` (`/Game/Blueprints/BP_Spline.Spline` (`self.spline Ref`)) 0.0 "World"))
  (`self.K2_SetActorTransform` (`KismetMathLibrary.MakeTransform` _returnvalue (`KismetMathLibrary.FindLookAtRotation` _returnvalue (`self.K2_GetActorLocation` (`self.LookAtTarget`)))))
  (`KismetSystemLibrary.Delay` 5.0)
  (if (`self.Test`)
    (`KismetSystemLibrary.ExecuteConsoleCommand` (`self.Start Profile Command`) null) ; Start Chart
  )
  (`TimelineComponent.SetPlayRate` (`self.Move Timeline`) (/ 1.0 (`self.Time to Complete (sec)`)))
  (bind (_direction _move) (`Timeline|Move Timeline`)
    (:`Update`
      (bind _returnvalue_2 (`SplineComponent.GetLocationAtDistanceAlongSpline` (`/Game/Blueprints/BP_Spline.Spline` (`self.spline Ref`)) (`KismetMathLibrary.Lerp` 0.0 (`SplineComponent.GetSplineLength` (`/Game/Blueprints/BP_Spline.Spline` (`self.spline Ref`))) _move) "World"))
      (`self.K2_SetActorTransform` (`KismetMathLibrary.MakeTransform` _returnvalue_2 (`KismetMathLibrary.FindLookAtRotation` _returnvalue_2 (`self.K2_GetActorLocation` (`self.LookAtTarget`)))))
      (if (>= _move 1.0)
        (`KismetSystemLibrary.Delay` 2.0)
        (if (`self.Test`)
          (`KismetSystemLibrary.ExecuteConsoleCommand` (`self.Stop Profile Command`) null))
        (`KismetSystemLibrary.QuitGame` null "Quit")))))

(fn `UserConstructionScript`)